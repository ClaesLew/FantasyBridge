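; Spline-driven fence actor that builds itself in the Construction Script, with no runtime logic.
; An InstancedStaticMesh places a Pole at every spline point, using the point's location and scale but zero local rotation.
; A SplineMeshComponent is added for each segment between neighboring points, bending the FenceBody mesh along the spline's locations and tangents.
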(event EventBeginPlay)

(event Collision|EventActorBeginOverlap
  (params (OtherActor :type Actor%20Object%20Reference)))

(event EventTick
  (params (DeltaSeconds :type Float%20%28single-precision%29)))

(fn ConstructionScript
  (Utilities|FlowControl|Sequence
    (:then_0
      (Components|StaticMesh|SetStaticMesh (Variables|Default|GetInstancedStaticMesh) (Variables|Default|GetPole)))
    (:then_1
      (for _index (range 0 (- (Spline|GetNumberOfSplinePoints (Variables|Default|GetSpline)) 1))
        (Components|InstancedStaticMesh|AddInstance (Variables|Default|GetInstancedStaticMesh) (Math|Transform|MakeTransform (.Location (Math|Transform|BreakTransform (Spline|GetTransformatSplinePoint (Variables|Default|GetSpline) _index "Local" true))) "0, 0, 0" (.Scale (Math|Transform|BreakTransform (Spline|GetTransformatSplinePoint (Variables|Default|GetSpline) _index "Local" true)))))))
    (:then_2
      (for _index_2 (range 0 (- (Spline|GetNumberOfSplinePoints (Variables|Default|GetSpline)) 2))
        (bind _returnvalue (AddComponent|AddSplineMeshComponent false))
        (Components|StaticMesh|SetStaticMesh _returnvalue (Variables|Default|GetFenceBody))
        (SplineMesh|SetStartandEnd _returnvalue (.Location (Spline|GetLocationandTangentatSplinePoint (Variables|Default|GetSpline) _index_2 "Local")) (.Tangent (Spline|GetLocationandTangentatSplinePoint (Variables|Default|GetSpline) _index_2 "Local")) (.Location (Spline|GetLocationandTangentatSplinePoint (Variables|Default|GetSpline) (+ _index_2 1) "Local")) (.Tangent (Spline|GetLocationandTangentatSplinePoint (Variables|Default|GetSpline) (+ _index_2 1) "Local")) true :!class /Script/Engine.SplineMeshComponent)))))